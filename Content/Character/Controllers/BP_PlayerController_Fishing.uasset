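; Player controller for the fishing character that caches the player's BP_Character on BeginPlay and handles menu, item and debug input.
; Escape creates and shows a pause widget, or resumes it when MenuOpen is set, which this graph never sets itself.
; ControlClick forwards clicks to the character's equipped EquipableActor.
; The 2 key advances FishingQuest when the game mode's Debug flag is on.
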(event `Key|Two`
  (params (Key :type "Key Structure" :default "AnyKey"))
  (:`Pressed`
    (bind _game_mode (`/Game/Functions/ActorMacros.Get Game Mode`)
      (:`Success`
        (if (`/Game/Gamemode/DefaultGameMode.Debug` _game_mode)
          (`/Game/Character/BP_Character.Advance Quest` (`self.My Character`) "FishingQuest"))))))

(event `self.ReceiveBeginPlay`
  (bind _asbp_character (cast `/Game/Character/BP_Character` (`GameplayStatics.GetPlayerCharacter` 0)))
  (set `self.My Character` _asbp_character))

(event `self.ReceiveTick`
  (params (DeltaSeconds :type "Float (single-precision)")))

(event `Toggle Controls`)

(event `InputAction|Escape`
  (params (Key :type "Key Structure" :default "AnyKey"))
  (:`Pressed`
    (if (`self.Menu Open`)
      (`/Game/HUD/Menus/Pause/PauseWidget.On Resume` (stale _returnvalue))
      (else
        (bind _returnvalue (`|CreateWidget` "/Game/HUD/Menus/Pause/PauseWidget.PauseWidget_C"))
        (`UserWidget.AddToViewport` _returnvalue 0)))))

(fn `Control Click`
  (returns (Success :type Boolean))
  (bind _asequipable_actor (cast `/Game/UsableActor/Inventory/EquipableActor` (`.Item_5_6E63FCE34F1BB2100A374F9CAAC7609A` (break `/Game/UsableActor/Inventory/Structs/InventoryStruct` (`/Game/Character/BP_Character.EquipedItem` (`self.My Character`)))))
    (:`then`
      (`/Game/UsableActor/Inventory/EquipableActor.onClick` _asequipable_actor))
    (:`CastFailed`
      _))
  (return true))

(fn `UserConstructionScript`)