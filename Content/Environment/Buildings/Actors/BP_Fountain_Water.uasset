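; Fountain water actor that reveals and raises the fountain's water when the final quest completes.
; On BeginPlay it binds to the DefaultGameMode's final-quest event and caches every BP_Fountain_Ripples actor.
; On trigger it unhides water and ripples, then a timeline lifts both by a fixed step per update up to a maximum.
; It calls OnWaterRiseComplete on the game mode at that limit and also when the timeline finishes.
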(event `self.ReceiveBeginPlay`
  ;[1 1 1] Begin Play: Set Gamemode, Bind Final Quest Complete to Gamemode.DoOnFinalQuestComplete, set Initial Variables, get all Fountain Ripples
  (bind _asdefault_game_mode (cast `/Game/Gamemode/DefaultGameMode` (`GameplayStatics.GetGameMode`)))
  (set `self.Game Mode` _asdefault_game_mode)
  (add `/Game/Gamemode/DefaultGameMode.Do On Final Quest Complete` _asdefault_game_mode (delegate `Final Quest Complete`))
  (set `self.Initial Z Offset` (.z (`SceneComponent.K2_GetComponentLocation` (`self.Water`))))
  (bind _outactors (`GameplayStatics.GetAllActorsOfClass` "/Game/Environment/Buildings/Actors/BP_Fountain_Ripples.BP_Fountain_Ripples_C"))
  (set `self.Fountain Ripples` _outactors))

(event `Final Quest Complete`
  ;[1 1 1] Begin Play: Set Gamemode, Bind Final Quest Complete to Gamemode.DoOnFinalQuestComplete, set Initial Variables, get all Fountain Ripples
  (`self.On Show`))

(event `On Show`
  (bind _returnvalue (`KismetMathLibrary.MakeVector` 0.0 0.0 0.01))
  ;[1 1 1] On Show: Show Water, Spouts, and Ripples, then raise water and ripples
  (if (not (`self.Has Completed`))
    (`self.Turn On Ripples`
      (:`Completed`
        (set `self.Running Z Change` 0.0)
        (set `self.Has Trigged Finished Water Rise` false)
        (`SceneComponent.SetHiddenInGame` (`self.Water`) false false)
        (`Timeline|Move Upwards` :!via `PlayFromStart`
          (:`Update`
            (if (< (`self.Running Z Change`) (`self.Max Z Change`))
              ;;[1 1 1] Raise Water and Ripples
              (set `self.Running Z Change` (+ (`self.Running Z Change`) 0.01))
              (`SceneComponent.K2_AddLocalOffset` (`self.Water`) _returnvalue false false)
              (`self.Add Offset To Ripples` _returnvalue)
              (else
                ;;[1 1 1] Call Water Rise Complete
                (if (not (`self.Has Trigged Finished Water Rise`))
                  (`/Game/Gamemode/DefaultGameMode.On Water Rise Complete` (`self.Game Mode`) :!label _label)
                  (set `self.Has Trigged Finished Water Rise` true)))))
          (:`Finished`
            (goto _label)))))))

(fn `UserConstructionScript`)